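; BP_BrokenDoor is a science lab sliding double door that opens and closes automatically when AutoDoor is set.
; Collision overlap begin and end events switch the AutoOpen and AutoClose flags, with no filter on the overlapping actor.
; Tick steps DoorPosition by a fixed amount per frame, so speed depends on frame rate, and slides the two LabDoor03 halves oppositely along local Y until a limit clears the flag.
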(event `self.Collision.OnComponentEndOverlap`
  (params (OverlappedComponent :type "PrimitiveComponent Object Reference") (OtherActor :type "Actor Object Reference") (OtherComp :type "PrimitiveComponent Object Reference") (OtherBodyIndex :type Integer))
  ;[0 0.3281 0] AutoOpenAndColseDoor
  (set `self.Auto Close` true)
  (set `self.Auto Open` false))

(event `self.Collision.OnComponentBeginOverlap`
  (params (OverlappedComponent :type "PrimitiveComponent Object Reference") (OtherActor :type "Actor Object Reference") (OtherComp :type "PrimitiveComponent Object Reference") (OtherBodyIndex :type Integer) (bFromSweep :type Boolean) (SweepResult :type "HitResult Structure (by ref)"))
  ;[0 0.3281 0] AutoOpenAndColseDoor
  (set `self.Auto Close` false)
  (set `self.Auto Open` true))

(event `self.ReceiveTick`
  (params (DeltaSeconds :type "Float (single-precision)"))
  (bind _doorposition (`self.DoorPosition`))
  (bind _doorposition_2 (`self.DoorPosition`))
  (bind _doorposition_3 (`self.DoorPosition`))
  ;[0 0.3281 0] AutoOpenAndColseDoor
  (if (`self.Auto Door`)
    (if (`self.Auto Open`)
      (`/Engine/EditorBlueprintResources/StandardMacros.CompareFloat` _doorposition_3 90.0
        (:`>`
          (set `self.DoorPosition` 90.0 :!label _label)
          (set `self.Auto Open` false))
        (:`==`
          (goto _label))
        (:`<`
          (set `self.DoorPosition` (+ _doorposition_3 4.0))
          (`SceneComponent.K2_SetRelativeLocation` (`self.LabDoor03B`) (`KismetMathLibrary.MakeVector` 0.0 _doorposition) false false :!label _label_2)
          (`SceneComponent.K2_SetRelativeLocation` (`self.LabDoor03A`) (`KismetMathLibrary.MakeVector` 0.0 (* _doorposition -1.0)) false false)))
      (elif (`self.Auto Close`)
        (`/Engine/EditorBlueprintResources/StandardMacros.CompareFloat` _doorposition_2
          (:`>`
            (set `self.DoorPosition` (- _doorposition_2 4.0))
            (goto _label_2))
          (:`==`
            _)
          (:`<`
            _))
        (set `self.DoorPosition` 0.0)
        (set `self.Auto Close` false)))))

(fn `UserConstructionScript`)