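; Player controller Blueprint that translates Enhanced Input actions into first-person movement, look and jump on player character 0.
; A custom event adds the IMC_Movement mapping context.
; Move input casts the character to BP_Body and uses only its first-person camera's yaw for forward and right directions, keeping pitch out of movement.
; Look input feeds controller yaw and pitch, and jump fires when its action starts.
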(event `CustomEvent`
  (`EnhancedInputSubsystemInterface.AddMappingContext` (subsystem `EnhancedInputLocalPlayerSubsystem`) "/Game/EurileneGene/Inputs/IMC_Movement.IMC_Movement" 0 (struct)))

(event `EnhancedInput|/Game/EurileneGene/Inputs/Action/IA_Moove`
  (params (ActionValue :type "Vector2D Structure") (ElapsedSeconds :type "Float (double-precision)") (TriggeredSeconds :type "Float (double-precision)") (InputAction :type "InputAction Object Reference" :default "/Game/EurileneGene/Inputs/Action/IA_Moove.IA_Moove"))
  (bind _returnvalue (`GameplayStatics.GetPlayerCharacter` 0))
  (:`Triggered`
    (bind _asbp_body (cast `/Game/EurileneGene/Core/BP_Body` _returnvalue))
    (bind (_returnvalue_roll _returnvalue_pitch _returnvalue_yaw) (`KismetMathLibrary.BreakRotator` (`SceneComponent.K2_GetComponentRotation` (`/Game/EurileneGene/Core/BP_Body.FirstPersonCamera` _asbp_body))))
    (`Pawn.AddMovementInput` _returnvalue (`KismetMathLibrary.GetForwardVector` (`KismetMathLibrary.MakeRotator` 0.0 0.0 _returnvalue_yaw)) ActionValue_X false)
    (`Pawn.AddMovementInput` _returnvalue (`KismetMathLibrary.GetRightVector` (`KismetMathLibrary.MakeRotator` 0.0 0.0 _returnvalue_yaw)) ActionValue_Y false)))

(event `EnhancedInput|/Game/EurileneGene/Inputs/Action/IA_Look`
  (params (ActionValue :type "Vector2D Structure") (ElapsedSeconds :type "Float (double-precision)") (TriggeredSeconds :type "Float (double-precision)") (InputAction :type "InputAction Object Reference" :default "/Game/EurileneGene/Inputs/Action/IA_Look.IA_Look"))
  (bind _returnvalue (`GameplayStatics.GetPlayerCharacter` 0))
  (:`Triggered`
    (`Pawn.AddControllerYawInput` _returnvalue ActionValue_X)
    (`Pawn.AddControllerPitchInput` _returnvalue ActionValue_Y)))

(event `EnhancedInput|/Game/EurileneGene/Inputs/Action/IA_Jump`
  (params (ActionValue :type Boolean) (ElapsedSeconds :type "Float (double-precision)") (TriggeredSeconds :type "Float (double-precision)") (InputAction :type "InputAction Object Reference" :default "/Game/EurileneGene/Inputs/Action/IA_Jump.IA_Jump"))
  (:`Started`
    (`Character.Jump` (`GameplayStatics.GetPlayerCharacter` 0))))

(fn `UserConstructionScript`)